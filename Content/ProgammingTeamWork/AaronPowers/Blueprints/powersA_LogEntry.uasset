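; Log entry actor that displays one logbook page as a widget: visual, spatial, physical, testimonial, table of contents, or a manual override.
; Construction spawns and fills the widget, feeding its render target into the Page's dynamic material unless it joins a logbook; BeginPlay destroys Page.
; Contents pages fill at BeginPlay, showing ten-chapter slices of the player's chapter list with locked names blank.
; Button and chapter hover/click events restyle elements and request redraws.
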(event Custom|ChapterButtonHover
  (params (index :type Integer))
  (bind _arraychaptertext (Variables|Default|GetarrayChapterText))
  (bind _output (Utilities|Array|Get(acopy) _arraychaptertext index))
  ;[1 1 1] Chapter Button Events
  (Utilities|IsValid _output
    (:Is%20Valid
      (TEXTFUNCTIONS|TextHover _output)
      (UserInterface|RequestRenderUpdate (Variables|Default|GetPageWidget)))))

(event Custom|UpdatePage
  ;[1 1 1] Update Widget Material
  (SETWIDGET|SetWidgetVariables)
  (UserInterface|RequestRenderUpdate (Variables|Default|GetPageWidget)))

(event Custom|NarrationButtonClick
  ;[1 1 1] Narration Button Events
  (BUTTONFUNCTIONS|ButtonClick (Variables|RUNTIMELOGREFERENCES|GetnarrationButton) true)
  (UserInterface|RequestRenderUpdate (Variables|Default|GetPageWidget)))

(event Custom|InformationButtonClick
  ;[1 1 1] Information Button Events
  (BUTTONFUNCTIONS|ButtonClick (Variables|RUNTIMELOGREFERENCES|GetinformationButton) false)
  (UserInterface|RequestRenderUpdate (Variables|Default|GetPageWidget)))

(event Custom|InformationButtonUnhover
  ;[1 1 1] Information Button Events
  (BUTTONFUNCTIONS|ButtonUnhover (Variables|RUNTIMELOGREFERENCES|GetinformationButton) false)
  (UserInterface|RequestRenderUpdate (Variables|Default|GetPageWidget)))

(event Custom|InformationButtonHover
  ;[1 1 1] Information Button Events
  (BUTTONFUNCTIONS|ButtonHover (Variables|RUNTIMELOGREFERENCES|GetinformationButton) false)
  (UserInterface|RequestRenderUpdate (Variables|Default|GetPageWidget)))

(event Custom|NarrationButtonHover
  ;[1 1 1] Narration Button Events
  (BUTTONFUNCTIONS|ButtonHover (Variables|RUNTIMELOGREFERENCES|GetnarrationButton) true)
  (UserInterface|RequestRenderUpdate (Variables|Default|GetPageWidget)))

(event Custom|NarrationButtonUnhover
  ;[1 1 1] Narration Button Events
  (BUTTONFUNCTIONS|ButtonUnhover (Variables|RUNTIMELOGREFERENCES|GetnarrationButton) true)
  (UserInterface|RequestRenderUpdate (Variables|Default|GetPageWidget)))

(event Custom|ChapterButtonClick
  (params (index :type Integer))
  (bind _arraychaptertext (Variables|Default|GetarrayChapterText))
  (bind _output (Utilities|Array|Get(acopy) _arraychaptertext index))
  ;[1 1 1] Chapter Button Events
  (Utilities|IsValid _output
    (:Is%20Valid
      (TEXTFUNCTIONS|TextClick _output)
      (UserInterface|RequestRenderUpdate (Variables|Default|GetPageWidget)))))

(event Custom|ChapterButtonUnhover
  (params (index :type Integer))
  (bind _arraychaptertext (Variables|Default|GetarrayChapterText))
  (bind _output (Utilities|Array|Get(acopy) _arraychaptertext index))
  ;[1 1 1] Chapter Button Events
  (Utilities|IsValid _output
    (:Is%20Valid
      (TEXTFUNCTIONS|TextUnhover _output)
      (UserInterface|RequestRenderUpdate (Variables|Default|GetPageWidget)))))

(event EventBeginPlay
  ;[1 1 1] Update Widget Material
  (Utilities|FlowControl|Delay 0.0)
  (if (Utilities|Enum|Equal(Enum) (Variables|LOGTYPE|GetwidgetType) "NewEnumerator4")
    (SETWIDGET|SetWidgetVariables))
  (Components|DestroyComponent (Variables|Default|GetPage))
  (UserInterface|RequestRenderUpdate (Variables|Default|GetPageWidget)))

(fn ConstructionScript
  (bind _widgettype (Variables|LOGTYPE|GetwidgetType))
  (CallFunction|SpawnWidgets _widgettype)
  (if (Utilities|Enum|Equal(Enum) _widgettype "NewEnumerator4")
    _
    (else
      (SETWIDGET|SetWidgetVariables)))
  (CallFunction|CreateMaterialInstance))

(fn CreateMaterialInstance
  ;[1 1 1] Prevent Creation of Additional Materials If Log Entry Is Going To Be Part Of Logbook
  (if (not (and (Utilities|IsValid (Variables|RUNTIMELOGREFERENCES|GetplayerCharacter)) (Variables|Default|GetpartOfPage)))
    ;[1 1 1] Set Parameter In Dynamic Material
    (bind _returnvalue (Rendering|Material|CreateDynamicMaterialInstance "/Game/ProgammingTeamWork/AaronPowers/Materials/testPageMaterial.testPageMaterial" "None" "None" :!class /Script/Engine.KismetMaterialLibrary))
    (bind _output_get (Variables|RUNTIMELOGREFERENCES|SetdynamicMaterial _returnvalue))
    (Rendering|Material|SetTextureParameterValue _output_get "FrontPageRenderTarget" (Class|WidgetComponent|GetRenderTarget (Variables|Default|GetPageWidget)))
    ;[1 1 1] Set Page To Dynamic Material
    (Rendering|Material|SetMaterial (Variables|Default|GetPage) 0 (Variables|RUNTIMELOGREFERENCES|GetdynamicMaterial))))

(fn SpawnWidgets
  (params (widgetType :type powersA_pageType%20Enum :default "NewEnumerator0"))
  ;[1 1 1] If The Widget Is A Custom One, Use It Instead
  (if (Utilities|IsValidClass (Variables|LOGTYPE|GetmanualOverrideWidget))
    (Variables|RUNTIMELOGREFERENCES|Setwidget (Variables|LOGTYPE|GetmanualOverrideWidget))
    (else
      ;[1 1 1] Set Widget Type To Spawn
      (switch Utilities|FlowControl|Switch|SwitchonpowersA_pageType widgetType
        (:NewEnumerator0
          (Variables|RUNTIMELOGREFERENCES|Setwidget "/Game/Developers/wapas/Visual_LogTemplate.Visual_LogTemplate_C"))
        (:NewEnumerator1
          (Variables|RUNTIMELOGREFERENCES|Setwidget "/Game/Developers/tyler/Collections/Spacial_LogTemplate.Spacial_LogTemplate_C"))
        (:NewEnumerator2
          (Variables|RUNTIMELOGREFERENCES|Setwidget "/Game/Developers/tyler/Collections/Physical_LogTemplate.Physical_LogTemplate_C"))
        (:NewEnumerator3
          (Variables|RUNTIMELOGREFERENCES|Setwidget "/Game/Developers/wapas/Testimonial_LogTemplate.Testimonial_LogTemplate_C"))
        (:NewEnumerator4
          (Variables|RUNTIMELOGREFERENCES|Setwidget "/Game/ProgammingTeamWork/AaronPowers/LogEntries/tableOfContents_LogTemplate.tableOfContents_LogTemplate_C")))))
  ;[1 1 1] Spawn Widget, Set to Ref, and Set Widget Component To Render Widget
  (bind _returnvalue (UserInterface|CreateWidget (Variables|RUNTIMELOGREFERENCES|Getwidget)))
  (bind _output_get (Variables|RUNTIMELOGREFERENCES|SetwidgetRef _returnvalue))
  (UserInterface|SetWidget (Variables|Default|GetPageWidget) _output_get)
  (return))

(fn SetWidgetVariables
  (bind _widgetref (Variables|RUNTIMELOGREFERENCES|GetwidgetRef))
  ;[1 1 1] If The Widget Is A Manually Made One, Skip The Process Of Setting Widget Variables
  (if (Utilities|IsValidClass (Variables|LOGTYPE|GetmanualOverrideWidget))
    (return)
    (else
      ;[1 1 1] Set Front Widget Variables Based On Widget Type
      (switch Utilities|FlowControl|Switch|SwitchonpowersA_pageType (Variables|LOGTYPE|GetwidgetType)
        (:NewEnumerator0
          (SETWIDGET|SetVisualPageWidgetVariables _widgetref))
        (:NewEnumerator1
          (SETWIDGET|SetSpacialPageWidgetVariables _widgetref))
        (:NewEnumerator2
          (SETWIDGET|SetPhysicalPageWidgetVariables _widgetref))
        (:NewEnumerator3
          (SETWIDGET|SetTestimonialPageWidgetVariables _widgetref))
        (:NewEnumerator4
          (SETWIDGET|TABLEOFCONTENTS|SetTableOfContentsWidgetVariables _widgetref)))
      (return))))

(fn SetVisualPageWidgetVariables
  (params (visualWidget :type User%20Widget%20Object%20Reference))
  (bind _asvisual_log_template (Utilities|Casting|CastToVisual_LogTemplate visualWidget))
  ;[1 1 1] Set Visual Log Variables
  (Rendering|Components|TextRender|SetText (Variables|/Game/Developers/wapas/Visual_LogTemplate.Visual_LogTemplate_C|GetDeckNameInfo _asvisual_log_template) (Variables|LOGSETTINGS|GetdeckNameInfo))
  (Rendering|Components|TextRender|SetText (Variables|/Game/Developers/wapas/Visual_LogTemplate.Visual_LogTemplate_C|GetPageTitle _asvisual_log_template) (Variables|LOGSETTINGS|GetpageTitle))
  (Rendering|Components|TextRender|SetText (Variables|/Game/Developers/wapas/Visual_LogTemplate.Visual_LogTemplate_C|GetPhotographerInfo _asvisual_log_template) (Variables|LOGSETTINGS|VISUAL|GetphotographerInfo))
  (Rendering|Components|TextRender|SetText (Variables|/Game/Developers/wapas/Visual_LogTemplate.Visual_LogTemplate_C|GetTakenInfo _asvisual_log_template) (Variables|LOGSETTINGS|VISUAL|GettakenInfo))
  (Appearance|SetBrushfromTexture (Variables|/Game/Developers/wapas/Visual_LogTemplate.Visual_LogTemplate_C|GetVisualImage _asvisual_log_template) (Variables|LOGSETTINGS|VISUAL|GetvisualImage) false)
  ;[1 1 1] Set Button Variables
  (Variables|RUNTIMELOGREFERENCES|SetnarrationButton (Variables|/Game/Developers/wapas/Visual_LogTemplate.Visual_LogTemplate_C|GetNarrationButton _asvisual_log_template))
  (Variables|RUNTIMELOGREFERENCES|SetinformationButton (Variables|/Game/Developers/wapas/Visual_LogTemplate.Visual_LogTemplate_C|GetInformationButton _asvisual_log_template)))

(fn SetSpacialPageWidgetVariables
  (params (spacialWidget :type User%20Widget%20Object%20Reference))
  (bind _asspacial_log_template (Utilities|Casting|CastToSpacial_LogTemplate spacialWidget))
  ;[1 1 1] Set Spacial Log Variables
  (Rendering|Components|TextRender|SetText (Variables|/Game/Developers/tyler/Collections/Spacial_LogTemplate.Spacial_LogTemplate_C|GetDeckNameInfo _asspacial_log_template) (Variables|LOGSETTINGS|GetdeckNameInfo))
  (Rendering|Components|TextRender|SetText (Variables|/Game/Developers/tyler/Collections/Spacial_LogTemplate.Spacial_LogTemplate_C|GetPageTitle _asspacial_log_template) (Variables|LOGSETTINGS|GetpageTitle))
  (Rendering|Components|TextRender|SetText (Variables|/Game/Developers/tyler/Collections/Spacial_LogTemplate.Spacial_LogTemplate_C|GetMainUseInfo _asspacial_log_template) (Variables|LOGSETTINGS|SPACIAL|GetmainUseInfo))
  (Rendering|Components|TextRender|SetText (Variables|/Game/Developers/tyler/Collections/Spacial_LogTemplate.Spacial_LogTemplate_C|GetAccessInfo _asspacial_log_template) (Variables|LOGSETTINGS|SPACIAL|GetaccessInfo))
  (Rendering|Components|TextRender|SetText (Variables|/Game/Developers/tyler/Collections/Spacial_LogTemplate.Spacial_LogTemplate_C|GetFlooringInfo _asspacial_log_template) (Variables|LOGSETTINGS|SPACIAL|GetflooringInfo))
  (Appearance|SetBrushfromTexture (Variables|/Game/Developers/tyler/Collections/Spacial_LogTemplate.Spacial_LogTemplate_C|GetSpacialImage _asspacial_log_template) (Variables|LOGSETTINGS|SPACIAL|GetspacialImage) false)
  ;[1 1 1] Set Button Variables
  (Variables|RUNTIMELOGREFERENCES|SetnarrationButton (Variables|/Game/Developers/tyler/Collections/Spacial_LogTemplate.Spacial_LogTemplate_C|GetNarrationButton _asspacial_log_template))
  (Variables|RUNTIMELOGREFERENCES|SetinformationButton (Variables|/Game/Developers/tyler/Collections/Spacial_LogTemplate.Spacial_LogTemplate_C|GetInformationButton _asspacial_log_template)))

(fn SetPhysicalPageWidgetVariables
  (params (physicalWidget :type User%20Widget%20Object%20Reference))
  (bind _asphysical_log_template (Utilities|Casting|CastToPhysical_LogTemplate physicalWidget))
  ;[1 1 1] Set Physical Log Variables
  (Rendering|Components|TextRender|SetText (Variables|/Game/Developers/tyler/Collections/Physical_LogTemplate.Physical_LogTemplate_C|GetDeckNameInfo _asphysical_log_template) (Variables|LOGSETTINGS|GetdeckNameInfo))
  (Rendering|Components|TextRender|SetText (Variables|/Game/Developers/tyler/Collections/Physical_LogTemplate.Physical_LogTemplate_C|GetPageTitle _asphysical_log_template) (Variables|LOGSETTINGS|GetpageTitle))
  (Rendering|Components|TextRender|SetText (Variables|/Game/Developers/tyler/Collections/Physical_LogTemplate.Physical_LogTemplate_C|GetManufacturerInfo _asphysical_log_template) (Variables|LOGSETTINGS|PHYSICAL|GetmanufacturerInfo))
  (Rendering|Components|TextRender|SetText (Variables|/Game/Developers/tyler/Collections/Physical_LogTemplate.Physical_LogTemplate_C|GetMaterialInfo _asphysical_log_template) (Variables|LOGSETTINGS|PHYSICAL|GetmaterialsInfo))
  (Rendering|Components|TextRender|SetText (Variables|/Game/Developers/tyler/Collections/Physical_LogTemplate.Physical_LogTemplate_C|GetDimensionsInfo _asphysical_log_template) (Variables|LOGSETTINGS|PHYSICAL|GetdimensionsInfo))
  (Rendering|Components|TextRender|SetText (Variables|/Game/Developers/tyler/Collections/Physical_LogTemplate.Physical_LogTemplate_C|GetTypeInfo _asphysical_log_template) (Variables|LOGSETTINGS|PHYSICAL|GettypeInfo))
  (Appearance|SetBrushfromTexture (Variables|/Game/Developers/tyler/Collections/Physical_LogTemplate.Physical_LogTemplate_C|GetPhysicalImage _asphysical_log_template) (Variables|LOGSETTINGS|PHYSICAL|GetphysicalImage) false)
  ;[1 1 1] Set Button Variables
  (Variables|RUNTIMELOGREFERENCES|SetnarrationButton (Variables|/Game/Developers/tyler/Collections/Physical_LogTemplate.Physical_LogTemplate_C|GetNarrationButton _asphysical_log_template))
  (Variables|RUNTIMELOGREFERENCES|SetinformationButton (Variables|/Game/Developers/tyler/Collections/Physical_LogTemplate.Physical_LogTemplate_C|GetInformationButton _asphysical_log_template)))

(fn SetTestimonialPageWidgetVariables
  (params (testimonialWidget :type User%20Widget%20Object%20Reference))
  (bind _astestimonial_log_template (Utilities|Casting|CastToTestimonial_LogTemplate testimonialWidget))
  ;[1 1 1] Set Testimonial Log Variables
  (Rendering|Components|TextRender|SetText (Variables|/Game/Developers/wapas/Testimonial_LogTemplate.Testimonial_LogTemplate_C|GetDeckNameInfo _astestimonial_log_template) (Variables|LOGSETTINGS|GetdeckNameInfo))
  (Rendering|Components|TextRender|SetText (Variables|/Game/Developers/wapas/Testimonial_LogTemplate.Testimonial_LogTemplate_C|GetpageTitle _astestimonial_log_template) (Variables|LOGSETTINGS|GetpageTitle))
  (Rendering|Components|TextRender|SetText (Variables|/Game/Developers/wapas/Testimonial_LogTemplate.Testimonial_LogTemplate_C|GetAgeInfo _astestimonial_log_template) (Variables|TESTIMONIAL|GetageInfo))
  (Rendering|Components|TextRender|SetText (Variables|/Game/Developers/wapas/Testimonial_LogTemplate.Testimonial_LogTemplate_C|GetClassInfo _astestimonial_log_template) (Variables|TESTIMONIAL|GetclassInfo))
  (Rendering|Components|TextRender|SetText (Variables|/Game/Developers/wapas/Testimonial_LogTemplate.Testimonial_LogTemplate_C|GetBirthplaceInfo _astestimonial_log_template) (Variables|TESTIMONIAL|GetbirthplaceInfo))
  (Rendering|Components|TextRender|SetText (Variables|/Game/Developers/wapas/Testimonial_LogTemplate.Testimonial_LogTemplate_C|GetDestinationInfo _astestimonial_log_template) (Variables|TESTIMONIAL|GetdestinationInfo))
  (Appearance|SetBrushfromTexture (Variables|/Game/Developers/wapas/Testimonial_LogTemplate.Testimonial_LogTemplate_C|GetTestimonialImage _astestimonial_log_template) (Variables|TESTIMONIAL|GettestimonialImage) false)
  ;[1 1 1] Set Button Variables
  (Variables|RUNTIMELOGREFERENCES|SetnarrationButton (Variables|/Game/Developers/wapas/Testimonial_LogTemplate.Testimonial_LogTemplate_C|GetNarrationButton _astestimonial_log_template))
  (Variables|RUNTIMELOGREFERENCES|SetinformationButton (Variables|/Game/Developers/wapas/Testimonial_LogTemplate.Testimonial_LogTemplate_C|GetInformationButton _astestimonial_log_template)))

(fn ButtonHover
  (params (buttonImage :type Image%20Object%20Reference) (isNarration :type Boolean))
  (if isNarration
    (Appearance|SetBrushfromTexture buttonImage "/Game/Developers/tyler/Collections/Log_Book_Assets/Log_Book_Assets/icons/white/play_icon.play_icon" false)
    (Appearance|SetColorandOpacity buttonImage "(R=1.000000,G=1.000000,B=1.000000,A=1.000000)" :!class /Script/UMG.Image)
    (else
      (Appearance|SetBrushfromTexture buttonImage "/Game/Developers/tyler/Collections/Log_Book_Assets/Log_Book_Assets/icons/white/source_icon.source_icon" false)
      (Appearance|SetColorandOpacity buttonImage "(R=1.000000,G=1.000000,B=1.000000,A=1.000000)" :!class /Script/UMG.Image))))

(fn ButtonUnhover
  (params (buttonImage :type Image%20Object%20Reference) (isNarration :type Boolean))
  (if isNarration
    (Appearance|SetBrushfromTexture buttonImage "/Game/Developers/tyler/Collections/Log_Book_Assets/Log_Book_Assets/icons/color/play_icon.play_icon" false)
    (Appearance|SetColorandOpacity buttonImage "(R=1.000000,G=1.000000,B=1.000000,A=1.000000)" :!class /Script/UMG.Image)
    (else
      (Appearance|SetBrushfromTexture buttonImage "/Game/Developers/tyler/Collections/Log_Book_Assets/Log_Book_Assets/icons/color/source_icon.source_icon" false)
      (Appearance|SetColorandOpacity buttonImage "(R=1.000000,G=1.000000,B=1.000000,A=1.000000)" :!class /Script/UMG.Image))))

(fn ButtonClick
  (params (buttonImage :type Image%20Object%20Reference) (isNarration :type Boolean))
  (if isNarration
    (Appearance|SetBrushfromTexture buttonImage "/Game/Developers/tyler/Collections/Log_Book_Assets/Log_Book_Assets/icons/color/play_icon.play_icon" false)
    (Appearance|SetColorandOpacity buttonImage "(R=0.500000,G=0.500000,B=0.500000,A=1.000000)" :!class /Script/UMG.Image)
    (else
      (Appearance|SetBrushfromTexture buttonImage "/Game/Developers/tyler/Collections/Log_Book_Assets/Log_Book_Assets/icons/color/source_icon.source_icon" false)
      (Appearance|SetColorandOpacity buttonImage "(R=0.500000,G=0.500000,B=0.500000,A=1.000000)" :!class /Script/UMG.Image))))

(fn SetTableOfContentsWidgetVariables
  (params (tableOfContentsWidget :type User%20Widget%20Object%20Reference))
  ;[1 1 1] Generate Array Of The Chapter Texts, and Set The Text Variables For Each
  (SETWIDGET|TABLEOFCONTENTS|CreateTableOfContentsTextArray tableOfContentsWidget)
  (SETWIDGET|TABLEOFCONTENTS|SetChapterVariables))

(fn SetPageNumberText
  (bind _widgetref (Variables|RUNTIMELOGREFERENCES|GetwidgetRef))
  (bind _pagenumber (Variables|Default|GetpageNumber))
  (bind _returnvalue (Utilities|String|ToString(Integer) _pagenumber))
  (bind _returnvalue_2 (Utilities|String|Append "PG. " _returnvalue))
  (bind _returnvalue_3 (Utilities|Text|ToText(String) _returnvalue_2))
  (switch Utilities|FlowControl|Switch|SwitchonpowersA_pageType (Variables|LOGTYPE|GetwidgetType)
    (:NewEnumerator0
      ;[1 1 1] Set The Page Number On The Different Log Types
      (bind _asvisual_log_template (Utilities|Casting|CastToVisual_LogTemplate _widgetref))
      (Rendering|Components|TextRender|SetText (Variables|/Game/Developers/wapas/Visual_LogTemplate.Visual_LogTemplate_C|GetPageNumber _asvisual_log_template) _returnvalue_3))
    (:NewEnumerator1
      (bind _asspacial_log_template (Utilities|Casting|CastToSpacial_LogTemplate _widgetref))
      (Rendering|Components|TextRender|SetText (Variables|/Game/Developers/tyler/Collections/Spacial_LogTemplate.Spacial_LogTemplate_C|GetPageNumber _asspacial_log_template) _returnvalue_3))
    (:NewEnumerator2
      (bind _asphysical_log_template (Utilities|Casting|CastToPhysical_LogTemplate _widgetref))
      (Rendering|Components|TextRender|SetText (Variables|/Game/Developers/tyler/Collections/Physical_LogTemplate.Physical_LogTemplate_C|GetPageNumber _asphysical_log_template) _returnvalue_3))
    (:NewEnumerator3
      (bind _astestimonial_log_template (Utilities|Casting|CastToTestimonial_LogTemplate _widgetref))
      (Rendering|Components|TextRender|SetText (Variables|/Game/Developers/wapas/Testimonial_LogTemplate.Testimonial_LogTemplate_C|GetPageNumber _astestimonial_log_template) _returnvalue_3))
    (:NewEnumerator4
      (bind _astable_of_contents_log_template (Utilities|Casting|CastTotableOfContents_LogTemplate _widgetref))
      (Rendering|Components|TextRender|SetText (Variables|/Game/ProgammingTeamWork/AaronPowers/LogEntries/tableOfContents_LogTemplate.tableOfContents_LogTemplate_C|GetPageNumber _astable_of_contents_log_template) _returnvalue_3))))

(fn SetChapterVariables
  (bind _playercharacter (Variables|RUNTIMELOGREFERENCES|GetplayerCharacter))
  (bind _pagenumber (Variables|Default|GetpageNumber))
  (bind _playercharacter_2 (Variables|RUNTIMELOGREFERENCES|GetplayerCharacter))
  (bind _playercharacter_3 (Variables|RUNTIMELOGREFERENCES|GetplayerCharacter))
  (bind _returnvalue (- _pagenumber 1))
  (bind _firsttableofcontents (Variables|/Game/ProgammingTeamWork/AaronPowers/Blueprints/powersA_FirstPersonCharacter.powersA_FirstPersonCharacter_C|GetfirstTableOfContents _playercharacter_2))
  (bind _chapterref (Variables|/Game/ProgammingTeamWork/AaronPowers/Blueprints/powersA_FirstPersonCharacter.powersA_FirstPersonCharacter_C|GetchapterRef _playercharacter))
  (bind _unlockedpagesref (Variables|/Game/ProgammingTeamWork/AaronPowers/Blueprints/powersA_FirstPersonCharacter.powersA_FirstPersonCharacter_C|GetunlockedPagesRef _playercharacter_3))
  (bind _returnvalue_2 (- _returnvalue _firsttableofcontents))
  (bind _returnvalue_3 (* _returnvalue_2 10))
  ;[1 1 1] Get The Section of Chapters That This Table Of Contents Page Should Be Showing
  (for _index (range _returnvalue_3 (+ _returnvalue_3 9))
    ;[1 1 1] Set Text Per Each Chapter (Only If The Chapter Is Unlocked
    (if (Utilities|Array|IsValidIndex _chapterref _index)
      (if (.isChapterFront (Utilities|Struct|BreakpowersA_chapterInfo (Utilities|Array|Get(acopy) _chapterref _index)))
        (if (Utilities|Array|Get(acopy) _unlockedpagesref (* (.chapterPage (Utilities|Struct|BreakpowersA_chapterInfo (Utilities|Array|Get(acopy) _chapterref _index))) 2))
          (Rendering|Components|TextRender|SetText (Utilities|Array|Get(acopy) (Variables|Default|GetarrayChapterText) (- _index _returnvalue_3)) (Utilities|Text|ToText(String) (.chapterName (Utilities|Struct|BreakpowersA_chapterInfo (Utilities|Array|Get(acopy) _chapterref _index)))) :!label _label)
          (else
            (Rendering|Components|TextRender|SetText (Utilities|Array|Get(acopy) (Variables|Default|GetarrayChapterText) (- _index _returnvalue_3)) "" :!label _label_2)))
        (elif (Utilities|Array|Get(acopy) _unlockedpagesref (- (* (.chapterPage (Utilities|Struct|BreakpowersA_chapterInfo (Utilities|Array|Get(acopy) _chapterref _index))) 2) 1))
          (goto _label)
          (else
            (goto _label_2))))
      (else
        (Rendering|Components|TextRender|SetText (Utilities|Array|Get(acopy) (Variables|Default|GetarrayChapterText) (- _index _returnvalue_3)) "")))))

(fn CreateTableOfContentsTextArray
  (params (TableOfContentsWidget :type User%20Widget%20Object%20Reference))
  (bind _arraychaptertext (Variables|Default|GetarrayChapterText))
  (Utilities|Array|Clear (Variables|Default|GetarrayChapterText))
  ;[1 1 1] Collect All Chapter Text and Dump Into Array
  (bind _astable_of_contents_log_template (Utilities|Casting|CastTotableOfContents_LogTemplate TableOfContentsWidget))
  (Utilities|Array|Add _arraychaptertext (Variables|/Game/ProgammingTeamWork/AaronPowers/LogEntries/tableOfContents_LogTemplate.tableOfContents_LogTemplate_C|GetChapter1Text _astable_of_contents_log_template))
  (Utilities|Array|Add _arraychaptertext (Variables|/Game/ProgammingTeamWork/AaronPowers/LogEntries/tableOfContents_LogTemplate.tableOfContents_LogTemplate_C|GetChapter2Text _astable_of_contents_log_template))
  (Utilities|Array|Add _arraychaptertext (Variables|/Game/ProgammingTeamWork/AaronPowers/LogEntries/tableOfContents_LogTemplate.tableOfContents_LogTemplate_C|GetChapter3Text _astable_of_contents_log_template))
  (Utilities|Array|Add _arraychaptertext (Variables|/Game/ProgammingTeamWork/AaronPowers/LogEntries/tableOfContents_LogTemplate.tableOfContents_LogTemplate_C|GetChapter4Text _astable_of_contents_log_template))
  (Utilities|Array|Add _arraychaptertext (Variables|/Game/ProgammingTeamWork/AaronPowers/LogEntries/tableOfContents_LogTemplate.tableOfContents_LogTemplate_C|GetChapter5Text _astable_of_contents_log_template))
  (Utilities|Array|Add _arraychaptertext (Variables|/Game/ProgammingTeamWork/AaronPowers/LogEntries/tableOfContents_LogTemplate.tableOfContents_LogTemplate_C|GetChapter6Text _astable_of_contents_log_template))
  (Utilities|Array|Add _arraychaptertext (Variables|/Game/ProgammingTeamWork/AaronPowers/LogEntries/tableOfContents_LogTemplate.tableOfContents_LogTemplate_C|GetChapter7Text _astable_of_contents_log_template))
  (Utilities|Array|Add _arraychaptertext (Variables|/Game/ProgammingTeamWork/AaronPowers/LogEntries/tableOfContents_LogTemplate.tableOfContents_LogTemplate_C|GetChapter8Text _astable_of_contents_log_template))
  (Utilities|Array|Add _arraychaptertext (Variables|/Game/ProgammingTeamWork/AaronPowers/LogEntries/tableOfContents_LogTemplate.tableOfContents_LogTemplate_C|GetChapter9Text _astable_of_contents_log_template))
  (Utilities|Array|Add _arraychaptertext (Variables|/Game/ProgammingTeamWork/AaronPowers/LogEntries/tableOfContents_LogTemplate.tableOfContents_LogTemplate_C|GetChapter10Text _astable_of_contents_log_template))
  (return))

(fn TextHover
  (params (buttonText :type Text%20Block%20Object%20Reference))
  (Appearance|SetColorandOpacity buttonText (LocalVariables|GethoverColor) :!class /Script/UMG.TextBlock))

(fn TextUnhover
  (params (buttonText :type Text%20Block%20Object%20Reference))
  (Appearance|SetColorandOpacity buttonText (LocalVariables|GetunhoverColor) :!class /Script/UMG.TextBlock))

(fn TextClick
  (params (buttonText :type Text%20Block%20Object%20Reference))
  (Appearance|SetColorandOpacity buttonText (LocalVariables|GetclickColor) :!class /Script/UMG.TextBlock))