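; A placeable log entry obtainer that unlocks a configured log entry for the player on interact.
; Begin and end look-at events track focus and cache the first-person character, and the actor handles the interact input itself.
; When interaction is allowed and no page is changing, it passes the entry class and index to the character, optionally destroying itself on success.
; A missing entry class prints an error.
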(event EventBeginLookingat
  ;[1 1 1] Is The Object Looked At?
  (bind _aspowers_a_first_person_character (Utilities|Casting|CastTopowersA_FirstPersonCharacter (Game|GetPlayerCharacter 0)))
  (Variables|Default|SetplayerCharacter _aspowers_a_first_person_character)
  (Variables|Default|SetisLookedAt true))

(event EventEndLookingat
  ;[1 1 1] Is The Object Looked At?
  (Variables|Default|SetisLookedAt false))

(event EventInputInteractPressed
  (params (NewParam :type Key%20Structure :default "None"))
  (bind _playercharacter (Variables|Default|GetplayerCharacter))
  ;[1 1 1] If the Player can Interact with the Log Entry Obtainer, and the Obtainer Has A Valid Class
  (if (Math|Boolean|ANDBoolean (Variables|Default|GetisLookedAt) (Variables|/Game/ProgammingTeamWork/AaronPowers/Blueprints/powersA_FirstPersonCharacter.powersA_FirstPersonCharacter_C|GetcanInteract _playercharacter) (not (Variables|/Game/ProgammingTeamWork/AaronPowers/Blueprints/powersA_FirstPersonCharacter.powersA_FirstPersonCharacter_C|GetpageChanging _playercharacter)))
    (if (Utilities|IsValidClass (Variables|Default|GetlogEntryUnlock))
      ;[1 1 1] Unlock The Log Entry
      (bind _wassuccessful (Default|ObtainLogEntry (Variables|Default|GetplayerCharacter) (Variables|Default|GetlogEntryUnlock) (Variables|Default|GetlogEntryIndexUnlock)))
      ;[1 1 1] Remove Actor
      (if (and _wassuccessful (Variables|Default|GetdestroyOnObtain))
        (Variables|/Game/ProgammingTeamWork/AaronPowers/Blueprints/powersA_FirstPersonCharacter.powersA_FirstPersonCharacter_C|SetobjectLookedAt (Variables|Default|GetplayerCharacter) 0)
        (Actor|DestroyActor))
      (else
        (Development|PrintString "ERROR!! THIS LOG ENTRY OBTAINER HAS NO LOG ENTRY SELECTED TO OBTAIN!!" true true "(R=1.000000,G=0.260123,B=0.280020,A=1.000000)" 5.0)))))

(fn ConstructionScript)