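; Two-sided book page actor that displays front and back log entries on a flippable page mesh.
; It spawns log-entry actors, labels their page numbers, and feeds their widget render targets into one dynamic material, with a fallback texture.
; Two zero-length delays before material assignment avoid blank pages.
; ChangePage destroys and respawns entries, UpdatePage refreshes them, and SetPageGradientFade drives each side's gradient reveal.
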(event Custom|UpdatePage
  ;[1 1 1] Update Page Variable
  (Default|UpdatePage (Variables|Default|GetfrontLogRef))
  (Default|UpdatePage (Variables|Default|GetbackLogRef))
  ;[1 1 1] Create the Material
  (CallFunction|UpdateMaterialInstance))

(event Custom|ChangePage
  ;[1 1 1] Delete Old Widgets For New Ones
  (CallFunction|ClearOldWidgets)
  ;[1 1 1] Spawns Two Log Entry Widgets (Front & Back)
  (CallFunction|SpawnWidgetReferences)
  ;[1 0 0] For some reason, we need TWO delays here for the material to update properly. First one is so the pages don't appear blank, and the second one keeps the pages from being blank for a single frame during the page flip animation.
  (Utilities|FlowControl|Delay 0.0)
  (Utilities|FlowControl|Delay 0.0)
  ;[1 1 1] Create the Material
  (CallFunction|UpdateMaterialInstance))

(event EventBeginPlay
  ;[1 1 1] Spawns Two Log Entry Widgets (Front & Back)
  (CallFunction|SpawnWidgetReferences)
  ;[1 0 0] For some reason, we need TWO delays here for the material to update properly. First one is so the pages don't appear blank, and the second one keeps the pages from being blank for a single frame during the page flip animation.
  (Utilities|FlowControl|Delay 0.0)
  (Utilities|FlowControl|Delay 0.0)
  ;[1 1 1] Create the Material
  (CallFunction|UpdateMaterialInstance))

(fn ConstructionScript)

(fn UpdateMaterialInstance
  (bind _frontlogref (Variables|Default|GetfrontLogRef))
  (bind _backlogref (Variables|Default|GetbackLogRef))
  ;[1 1 1] Create Material If None Exists-If One Does, Just Use Old Material
  (Utilities|IsValid (Variables|Default|GetdynamicMaterial)
    (:Is%20Valid
      _)
    (:Is%20Not%20Valid
      (bind _returnvalue (Rendering|Material|CreateDynamicMaterialInstance "/Game/ProgammingTeamWork/AaronPowers/Materials/testPageMaterial.testPageMaterial" "None" "None" :!class /Script/Engine.KismetMaterialLibrary))
      (Variables|Default|SetdynamicMaterial _returnvalue)))
  ;[1 1 1] Assign Render Textures To Dynamic Material Parameters
  (Utilities|IsValid _frontlogref
    (:Is%20Valid
      (Rendering|Material|SetTextureParameterValue (Variables|Default|GetdynamicMaterial) "FrontPageRenderTarget" (Class|WidgetComponent|GetRenderTarget (Variables|/Game/ProgammingTeamWork/AaronPowers/Blueprints/powersA_LogEntry.powersA_LogEntry_C|GetPageWidget _frontlogref))))
    (:Is%20Not%20Valid
      (Rendering|Material|SetTextureParameterValue (Variables|Default|GetdynamicMaterial) "FrontPageRenderTarget" "/Game/Developers/ahpow/Collections/Textures/bookSystem_renderTargetTemp.bookSystem_renderTargetTemp")))
  (Utilities|IsValid _backlogref
    (:Is%20Valid
      (Rendering|Material|SetTextureParameterValue (Variables|Default|GetdynamicMaterial) "BackPageRenderTarget" (Class|WidgetComponent|GetRenderTarget (Variables|/Game/ProgammingTeamWork/AaronPowers/Blueprints/powersA_LogEntry.powersA_LogEntry_C|GetPageWidget _backlogref))))
    (:Is%20Not%20Valid
      (Rendering|Material|SetTextureParameterValue (Variables|Default|GetdynamicMaterial) "BackPageRenderTarget" "/Game/ProgammingTeamWork/AaronPowers/Textures/bookSystem_renderTargetTemp.bookSystem_renderTargetTemp")))
  ;[1 1 1] Set Material To Page
  (Rendering|Material|SetMaterial (Variables|Default|GetPage) 0 (Variables|Default|GetdynamicMaterial)))

(fn SpawnWidgetReferences
  (bind _frontlogentry (Variables|Default|GetfrontLogEntry))
  (bind _backlogentry (Variables|Default|GetbackLogEntry))
  (bind _defaultsceneroot (Variables|Default|GetDefaultSceneRoot))
  (bind _returnvalue (Transformation|GetWorldTransform _defaultsceneroot))
  ;[1 1 1] Spawn Front Log Entry
  (if (Utilities|IsValidClass _frontlogentry)
    (bind _returnvalue_2 (Game|SpawnActorfromClass _frontlogentry _returnvalue "Undefined" 0 0))
    (bind _output_get (Variables|Default|SetfrontLogRef _returnvalue_2))
    (bind _pagenumtext (CallFunction|SetPageNumber false))
    (Variables|/Game/ProgammingTeamWork/AaronPowers/Blueprints/powersA_LogEntry.powersA_LogEntry_C|SetpageNumberVariable _output_get _pagenumtext)
    (Default|SetPageNumberText _output_get)
    (UserInterface|RequestRenderUpdate (Variables|/Game/ProgammingTeamWork/AaronPowers/Blueprints/powersA_LogEntry.powersA_LogEntry_C|GetPageWidget _output_get)))
  ;[1 1 1] Spawn Back Log Entry
  (if (Utilities|IsValidClass _backlogentry)
    (bind _returnvalue_3 (Game|SpawnActorfromClass _backlogentry _returnvalue "Undefined" 0 0))
    (bind _output_get_2 (Variables|Default|SetbackLogRef _returnvalue_3))
    (bind _pagenumtext_2 (CallFunction|SetPageNumber true))
    (Variables|/Game/ProgammingTeamWork/AaronPowers/Blueprints/powersA_LogEntry.powersA_LogEntry_C|SetpageNumberVariable _output_get_2 _pagenumtext_2)
    (Default|SetPageNumberText _output_get_2)
    (UserInterface|RequestRenderUpdate (Variables|/Game/ProgammingTeamWork/AaronPowers/Blueprints/powersA_LogEntry.powersA_LogEntry_C|GetPageWidget _output_get_2)))
  (return))

(fn ClearOldWidgets
  (bind _frontlogref (Variables|Default|GetfrontLogRef))
  (bind _backlogref (Variables|Default|GetbackLogRef))
  ;[1 1 1] Delete Old Log Entries (If Valid)
  (Utilities|IsValid _frontlogref
    (:Is%20Valid
      (Actor|DestroyActor _frontlogref)
      (Utilities|IsValid _backlogref
        (:Is%20Valid
          (Actor|DestroyActor _backlogref))))))

(fn SetPageNumber
  (params (isBackPage :type Boolean))
  (bind _pagenumber (Variables|Default|GetpageNumber))
  (bind _returnvalue (+ _pagenumber 1))
  ;[1 1 1] Is There A Valid Page Number
  (if (!= (+ (Variables|Default|GetpageNumber) 1) 0)
    ;[1 1 1] Is Front Or Back Page
    (if isBackPage
      ;[1 1 1] Back Page-Multiply Page # By 2
      (return (Utilities|Text|ToText(String) (Utilities|String|Append "PG. " (Utilities|String|ToString(Integer) (* _returnvalue 2)))))
      (else
        ;[1 1 1] Page Front- Multiply Page # By 2 And -1
        (return (Utilities|Text|ToText(String) (Utilities|String|Append "PG. " (Utilities|String|ToString(Integer) (- (* _returnvalue 2) 1)))))))
    (else
      (return "PG. NO"))))

(fn SetPageGradientFade
  (params (frontPage :type Boolean) (pageGradientFadeValue :type Float%20%28single-precision%29))
  (bind _dynamicmaterial (Variables|Default|GetdynamicMaterial))
  ;[1 1 1] Set Gradient Fade
  (if frontPage
    (Rendering|Material|SetScalarParameterValue _dynamicmaterial "FrontPageGradientReveal" pageGradientFadeValue :!class /Script/Engine.MaterialInstanceDynamic)
    (else
      (Rendering|Material|SetScalarParameterValue _dynamicmaterial "BackPageGradientReveal" pageGradientFadeValue :!class /Script/Engine.MaterialInstanceDynamic))))